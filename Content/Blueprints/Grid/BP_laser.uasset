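; BP_laser is a grid laser that turns 90 degrees in yaw on each TickTockClockMove event, fired when the player moves.
; Every Tick it line-traces on the Camera channel along the Cube's forward vector, draws the debug line and prints the hit actor's name.
; The debug line is the only live beam visual, as the Cascade beam and Niagara spawn chains are disconnected and never run.
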(event `self.ReceiveTick`
  (params (DeltaSeconds :type "Float (single-precision)"))
  (bind _returnvalue (`SceneComponent.K2_GetComponentLocation` (`self.Cube`)))
  ;[1 0.3984 0] Renders a line to show hitting
  (bind (_outhit _returnvalue_2) (`KismetSystemLibrary.LineTraceSingle` :`Start` _returnvalue :`End` (+ (* (`SceneComponent.GetForwardVector` (`self.Cube`)) 25000.0) _returnvalue) :`TraceChannel` "TraceTypeQuery2" :`DrawDebugType` "ForOneFrame"))
  (`KismetSystemLibrary.PrintString` (`KismetSystemLibrary.GetDisplayName` (`.HitActor` (`GameplayStatics.BreakHitResult` _outhit)))))

(event `self.ReceiveBeginPlay`)

(event `/Game/Blueprints/Grid/BPI_ClockButtons.Tick tock clock move`
  (bind (_returnvalue_roll _returnvalue_pitch _returnvalue_yaw) (`KismetMathLibrary.BreakRotator` (`SceneComponent.K2_GetComponentRotation` (`self.Cube`))))
  ;[1 0 0.8906] Everytime player moves, laser rotates
  (`SceneComponent.K2_SetWorldRotation` (`self.Cube`) (`KismetMathLibrary.MakeRotator` 0.0 0.0 (+ _returnvalue_yaw 90.0)) false false))

(fn `UserConstructionScript`)