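; Player character for a grid puzzle game that steps its cube a fixed distance per directional input, gated by a Tick-driven delay timer.
; Swept moves snap back to the original location when blocked, except forward and backward hits on two teleport actors.
; Each successful move resets the timer and sends a tick message to BPLaser.
; Pause input opens the pause menu; a four-way LineTrace check is defined but unused.
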(event `InputAction|Pause`
  (params (Key :type "Key Structure"))
  (:`Pressed`
    (bind _returnvalue (`|CreateWidget` "/Game/Widgets/W_PauseMenu.W_PauseMenu_C"))
    (`UserWidget.AddToViewport` _returnvalue 0)
    (set `PlayerController.bShowMouseCursor` true (`GameplayStatics.GetPlayerController` 0))))

(event `self.ReceiveTick`
  (params (DeltaSeconds :type "Float (single-precision)"))
  ;[1 0 0.4453] stops player form moving to try and not get laser zapped
  (set `self.MoveDelayTimer` (+ (`self.MoveDelayTimer`) DeltaSeconds)))

(event `InputAction|MoveBackwardsButton`
  (params (Key :type "Key Structure"))
  (bind _returnvalue (`GameplayStatics.GetPlayerPawn` 0))
  (bind _cube (`self.Cube`))
  (bind (_returnvalue_x _returnvalue_y _returnvalue_z) (`KismetMathLibrary.BreakVector` (`SceneComponent.K2_GetComponentLocation` _cube)))
  ;[0 1 0.9531] Moves player back
  (:`Pressed`
    (`self.CanMove`
      (:`CanMove`
        (bind _output_get (set `self.OriginalLocation` (`self.K2_GetActorLocation` _returnvalue)))
        (bind _sweephitresult (`SceneComponent.K2_SetWorldLocation` _cube (`KismetMathLibrary.MakeVector` (- _returnvalue_x (`self.MoveThisManySpaces`)) _returnvalue_y _returnvalue_z) true false))
        (if (`GameplayStatics.BreakHitResult` _sweephitresult)
          (if (or (== (`.HitActor` (`GameplayStatics.BreakHitResult` _sweephitresult)) (`self.Teleport1`)) (== (`self.Teleport2`) (`.HitActor` (`GameplayStatics.BreakHitResult` _sweephitresult))))
            (`self.MovieYesYumYUm` :!label _label)
            (else
              (`SceneComponent.K2_SetWorldLocation` (`Actor.RootComponent` _returnvalue) _output_get false false)))
          (else
            (goto _label)))))))

(event `InputAction|MoveForwardButton`
  (params (Key :type "Key Structure"))
  (bind _returnvalue (`GameplayStatics.GetPlayerPawn` 0))
  (bind _cube (`self.Cube`))
  (bind (_returnvalue_x _returnvalue_y _returnvalue_z) (`KismetMathLibrary.BreakVector` (`SceneComponent.K2_GetComponentLocation` _cube)))
  ;[1 0 0.4219] Moves player forward
  (:`Pressed`
    (`self.CanMove`
      (:`CanMove`
        (bind _output_get (set `self.OriginalLocation` (`self.K2_GetActorLocation` _returnvalue)))
        (bind _sweephitresult (`SceneComponent.K2_SetWorldLocation` _cube (`KismetMathLibrary.MakeVector` (+ _returnvalue_x (`self.MoveThisManySpaces`)) _returnvalue_y _returnvalue_z) true false))
        (if (`GameplayStatics.BreakHitResult` _sweephitresult)
          (if (or (== (`.HitActor` (`GameplayStatics.BreakHitResult` _sweephitresult)) (`self.Teleport1`)) (== (`self.Teleport2`) (`.HitActor` (`GameplayStatics.BreakHitResult` _sweephitresult))))
            ;;[0.8281 1 0] Awful check to see if it's a teleport which has been hit, and if it is, then the movement carries on as normal. There has got to be a better way to do it
            (`self.MovieYesYumYUm` :!label _label_2)
            (else
              (`SceneComponent.K2_SetWorldLocation` (`Actor.RootComponent` _returnvalue) _output_get false false)))
          (else
            (goto _label_2)))))))

(event `InputAction|Movement`
  (params (Key :type "Key Structure"))
  ;[0.8516 0 1] Each movement spins laser
)

(event `InputAction|MoveRight`
  (params (Key :type "Key Structure"))
  (bind _returnvalue (`GameplayStatics.GetPlayerPawn` 0))
  (bind _cube (`self.Cube`))
  (bind (_returnvalue_x _returnvalue_y _returnvalue_z) (`KismetMathLibrary.BreakVector` (`SceneComponent.K2_GetComponentLocation` _cube)))
  ;[0 0.6484 1] Moves player right
  (:`Pressed`
    (`self.CanMove`
      (:`CanMove`
        (bind _output_get (set `self.OriginalLocation` (`self.K2_GetActorLocation` _returnvalue)))
        (bind _sweephitresult (`SceneComponent.K2_SetWorldLocation` _cube (`KismetMathLibrary.MakeVector` _returnvalue_x (+ _returnvalue_y (`self.MoveThisManySpaces`)) _returnvalue_z) true false))
        (if (`GameplayStatics.BreakHitResult` _sweephitresult)
          (`SceneComponent.K2_SetWorldLocation` (`Actor.RootComponent` _returnvalue) _output_get false false)
          (else
            (`self.MovieYesYumYUm`)))))))

(event `InputAction|MoveLeft`
  (params (Key :type "Key Structure"))
  (bind _returnvalue (`GameplayStatics.GetPlayerPawn` 0))
  (bind _cube (`self.Cube`))
  (bind (_returnvalue_x _returnvalue_y _returnvalue_z) (`KismetMathLibrary.BreakVector` (`SceneComponent.K2_GetComponentLocation` _cube)))
  ;[0.6641 0 1] moves player left
  (:`Pressed`
    (`self.CanMove`
      (:`CanMove`
        (bind _output_get (set `self.OriginalLocation` (`self.K2_GetActorLocation` _returnvalue)))
        (bind _sweephitresult (`SceneComponent.K2_SetWorldLocation` _cube (`KismetMathLibrary.MakeVector` _returnvalue_x (- _returnvalue_y (`self.MoveThisManySpaces`)) _returnvalue_z) true false))
        (if (`GameplayStatics.BreakHitResult` _sweephitresult)
          (`SceneComponent.K2_SetWorldLocation` (`Actor.RootComponent` _returnvalue) _output_get false false)
          (else
            (`self.MovieYesYumYUm`)))))))

(fn `MovieYesYumYUm`
  (set `self.MoveDelayTimer` 0.0)
  (message `/Game/Blueprints/Grid/BPI_ClockButtons.Tick tock clock move` (`self.BP_laser`)))

(fn `UserConstructionScript`)