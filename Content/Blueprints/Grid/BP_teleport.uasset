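; BP_teleport is a grid teleporter cube that sends the player to another teleport in the level when touched.
; On BeginPlay it tints its cube purple through a dynamic material instance.
; A hit on the cube by the player pawn moves the player to a manually linked Teleport actor's location plus an instance-editable Direction offset, so they exit beside it.
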(event `self.ReceiveBeginPlay`
  ;[0.8281 0 1] Changes colour to purple
  (bind _returnvalue (`PrimitiveComponent.CreateDynamicMaterialInstance` (`self.Cube1`) 0 null "None"))
  (`MaterialInstanceDynamic.SetVectorParameterValue` _returnvalue "Color" (struct :`R` 0.348958 :`B` 0.327497 :`A` 1.0)))

(event `self.Cube1.OnComponentHit`
  (params (HitComponent :type "PrimitiveComponent Object Reference") (OtherActor :type "Actor Object Reference") (OtherComp :type "PrimitiveComponent Object Reference") (NormalImpulse :type "Vector Structure") (Hit :type "HitResult Structure (by ref)"))
  ;[0 0.5547 1] Checks if player touches teleport
  (if (== (`GameplayStatics.GetPlayerPawn` 0) OtherActor)
    ;[1 0.6328 0] Finds other teleport in level (manually, instance editable), and spits the player out in a (manual, instance editable) direction
    (`self.K2_SetActorLocation` (`self.Player`) (+ (`self.K2_GetActorLocation` (`self.Teleport`)) (`self.Direction`)) false false)))

(fn `UserConstructionScript`)