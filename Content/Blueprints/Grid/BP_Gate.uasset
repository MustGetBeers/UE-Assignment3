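; BP_Gate is a goal gate that counts collected keys and unblocks the way to the next level.
; PickUp increments the key count and, at GoalNumber, starts four timelines sinking the cubes, each update easing from the cube's current position, so movement accumulates.
; BeginPlay tints the cubes through dynamic material instances.
; When the player overlaps the Sphere, the camera fades out and LevelNameToLoad opens after a delay.
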(event `/Game/Blueprints/Grid/BPI_KeyPickUp.PickUp`
  (bind _cube (`self.Cube`))
  (bind _cube1 (`self.Cube1`))
  (bind _cube2 (`self.Cube2`))
  (bind _cube3 (`self.Cube3`))
  (bind _relativelocation (`SceneComponent.RelativeLocation` _cube))
  (bind _relativelocation_2 (`SceneComponent.RelativeLocation` _cube1))
  (bind _relativelocation_3 (`SceneComponent.RelativeLocation` _cube2))
  (bind _relativelocation_4 (`SceneComponent.RelativeLocation` _cube3))
  ;[0.03125 0 1] Adds keys when picked up and checks if it's enough to open up
  (bind _output_get (set `self.NumberOfKeys` (+ (`self.NumberOfKeys`) 1)))
  (if (== _output_get (`self.GoalNumber`))
    ;[0 0.8125 1] Horrific code for sliding down the goal-blocking blocks
    (`|ExecutionSequence`
      (:`then_0`
        (bind (_direction _newtrack_0) (`Timeline|Slide`)
          (:`Update`
            (`SceneComponent.K2_SetRelativeLocation` _cube (`|EaseFunction` "EaseIn" _newtrack_0 _relativelocation (+ _relativelocation (0.0 0.0 -20.0))) false false))))
      (:`then_1`
        (bind (_direction_2 _newtrack_0_2) (`Timeline|Timeline_0`)
          (:`Update`
            (`SceneComponent.K2_SetRelativeLocation` _cube1 (`|EaseFunction` "EaseIn" _newtrack_0_2 _relativelocation_2 (+ _relativelocation_2 (0.0 0.0 -20.0))) false false))))
      (:`then_2`
        (bind (_direction_3 _newtrack_0_3) (`Timeline|Timeline_1`)
          (:`Update`
            (`SceneComponent.K2_SetRelativeLocation` _cube2 (`|EaseFunction` "EaseIn" _newtrack_0_3 _relativelocation_3 (+ _relativelocation_3 (0.0 0.0 -20.0))) false false))))
      (:`then_3`
        (bind (_direction_4 _newtrack_0_4) (`Timeline|Timeline_2`)
          (:`Update`
            (`SceneComponent.K2_SetRelativeLocation` _cube3 (`|EaseFunction` "EaseIn" _newtrack_0_4 _relativelocation_4 (+ _relativelocation_4 (0.0 0.0 -20.0))) false false)))))))

(event `self.ReceiveBeginPlay`
  ;[1 0.4453 0] Changes colour of material
  (`|ExecutionSequence`
    (:`then_0`
      (bind _returnvalue (`PrimitiveComponent.CreateDynamicMaterialInstance` (`self.Cube`) 0 "/Game/Materials/Mat_basecolour.Mat_basecolour" "None"))
      (`MaterialInstanceDynamic.SetVectorParameterValue` _returnvalue "Color" (struct :`R` 0.432292 :`G` 0.416234 :`A` 1.0)))
    (:`then_1`
      (bind _returnvalue_2 (`PrimitiveComponent.CreateDynamicMaterialInstance` (`self.Cube1`) 0 "/Game/Materials/Mat_basecolour.Mat_basecolour" "None"))
      (`MaterialInstanceDynamic.SetVectorParameterValue` _returnvalue_2 "Color" (struct :`R` 0.434154 :`G` 0.417885 :`A` 1.0)))
    (:`then_2`
      (bind _returnvalue_3 (`PrimitiveComponent.CreateDynamicMaterialInstance` (`self.Cube2`) 0 "/Game/Materials/Mat_basecolour.Mat_basecolour" "None"))
      (`MaterialInstanceDynamic.SetVectorParameterValue` _returnvalue_3 "Color" (struct :`R` 0.434154 :`G` 0.417885 :`A` 1.0)))
    (:`then_3`
      (bind _returnvalue_4 (`PrimitiveComponent.CreateDynamicMaterialInstance` (`self.Cube3`) 0 "/Game/Materials/Mat_basecolour.Mat_basecolour" "None"))
      (`MaterialInstanceDynamic.SetVectorParameterValue` _returnvalue_4 "Color" (struct :`R` 0.434154 :`G` 0.417885 :`A` 1.0)))))

(event `self.Sphere.OnComponentBeginOverlap`
  (params (OverlappedComponent :type "PrimitiveComponent Object Reference") (OtherActor :type "Actor Object Reference") (OtherComp :type "PrimitiveComponent Object Reference") (OtherBodyIndex :type Integer) (bFromSweep :type Boolean) (SweepResult :type "HitResult Structure (by ref)"))
  (bind _returnvalue (`GameplayStatics.GetPlayerPawn` 0))
  ;[0.6641 0 1] Moves on to the next level
  (if (== _returnvalue OtherActor)
    (`PlayerCameraManager.StartCameraFade` :`self` (`GameplayStatics.GetPlayerCameraManager` 0) :`ToAlpha` 1.0 :`Duration` 1.0 :`bHoldWhenFinished` true)
    (`KismetSystemLibrary.Delay` 1.0)
    (`/Engine/EditorBlueprintResources/StandardMacros.IsValid` _returnvalue
      (:`Is Valid`
        (`GameplayStatics.OpenLevel` (`self.Level Name to load`))))))

(fn `UserConstructionScript`)