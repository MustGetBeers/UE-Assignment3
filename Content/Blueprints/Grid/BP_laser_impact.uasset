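; Laser hazard actor that destroys the player pawn when its beam hits it.
; Each tick a Camera-channel line trace along the forward vector sets the Niagara beam's end and shows the impact effect at blocking hits.
; The TickTockClockMove event turns the laser in quarter steps: one timeline pitches it upright, yaw advances 90 degrees, then a second timeline lowers it to horizontal.
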(event `self.ReceiveTick`
  (params (DeltaSeconds :type "Float (single-precision)"))
  (bind _returnvalue (`GameplayStatics.GetPlayerPawn` 0))
  (bind _returnvalue_2 (`self.K2_GetActorLocation`))
  (bind _returnvalue_3 (+ _returnvalue_2 (* (`self.GetActorForwardVector`) (`self.Distance`))))
  (set `self.Trace_end` _returnvalue_3)
  (bind _outhit (`KismetSystemLibrary.LineTraceSingle` :`Start` _returnvalue_2 :`End` _returnvalue_3 :`TraceChannel` "TraceTypeQuery2" :`DrawDebugType` "ForOneFrame"))
  (`|ExecutionSequence`
    (:`then_0`
      (set `self.bHit` (`GameplayStatics.BreakHitResult` _outhit))
      (set `self.Hit location` (`.Location` (`GameplayStatics.BreakHitResult` _outhit)))
      (`FXSystemComponent.SetVectorParameter` (`self.NiagaraLaser`) "Laser_end" (select `bool` (`self.bHit`) :`false` (`self.Trace_end`) :`true` (`self.Hit location`)))
      (`SceneComponent.SetVisibility` (`self.NiagaraLaserImpact`) (`self.bHit`) false)
      (`SceneComponent.K2_SetWorldLocation` (`self.NiagaraLaserImpact`) (`self.Hit location`) false false))
    (:`then_1`
      (if (`GameplayStatics.BreakHitResult` _outhit)
        (if (== _returnvalue (`.HitActor` (`GameplayStatics.BreakHitResult` _outhit)))
          (`self.K2_DestroyActor` _returnvalue))))))

(event `self.ReceiveBeginPlay`
  (`FXSystemComponent.SetColorParameter` (`self.NiagaraLaser`) "Laser_colour" (struct :`R` 1.0 :`G` 0.031044 :`A` 1.0))
  (`FXSystemComponent.SetColorParameter` (`self.NiagaraLaserImpact`) "Impact_colour" (struct :`R` 1.0 :`G` 0.236519 :`B` 0.066385 :`A` 1.0)))

(event `/Game/Blueprints/Grid/BPI_ClockButtons.Tick tock clock move`
  (bind (_rotation_roll _rotation_pitch _rotation_yaw) (`KismetMathLibrary.BreakRotator` (`self.Rotation`)))
  (bind (_rotation_roll_2 _rotation_pitch_2 _rotation_yaw_2) (`KismetMathLibrary.BreakRotator` (`self.Rotation`)))
  (bind (_rotation_roll_3 _rotation_pitch_3 _rotation_yaw_3) (`KismetMathLibrary.BreakRotator` (`self.Rotation`)))
  (bind (_rotation_roll_4 _rotation_pitch_4 _rotation_yaw_4) (`KismetMathLibrary.BreakRotator` (`self.Rotation`)))
  (bind (_rotation_roll_5 _rotation_pitch_5 _rotation_yaw_5) (`KismetMathLibrary.BreakRotator` (`self.Rotation`)))
  (bind (_startrotation_roll _startrotation_pitch) (`KismetMathLibrary.BreakRotator` (`self.StartRotation`)))
  (bind (_startrotation_roll_2 _startrotation_pitch_2) (`KismetMathLibrary.BreakRotator` (`self.StartRotation`)))
  (set `self.StartRotation` (`self.Rotation`))
  (set `self.Rotation` (`KismetMathLibrary.MakeRotator` 0.0 90.0 _rotation_yaw_3))
  (bind (_direction _goup) (`Timeline|GoUp` :!via `PlayFromStart`)
    (:`Update`
      (`self.K2_SetActorRotation` (`KismetMathLibrary.MakeRotator` 0.0 (`KismetMathLibrary.Lerp` _startrotation_pitch _rotation_pitch_5 _goup) _rotation_yaw_5)))
    (:`Finished`
      (bind _output_get (set `self.Rotation` (`KismetMathLibrary.MakeRotator` 0.0 90.0 (`KismetMathLibrary.Conv_IntToDouble` (mod (`KismetMathLibrary.Round` (+ _rotation_yaw_2 90.0)) 360)))))
      (`self.K2_SetActorRotation` _output_get)
      (set `self.StartRotation` _output_get)
      (set `self.Rotation` (`KismetMathLibrary.MakeRotator` 0.0 0.0 _rotation_yaw))
      (bind (_direction_2 _ggodown) (`Timeline|GoDown` :!via `PlayFromStart`)
        (:`Update`
          (`self.K2_SetActorRotation` (`KismetMathLibrary.MakeRotator` 0.0 (`KismetMathLibrary.Lerp` _startrotation_pitch_2 _rotation_pitch_4 _ggodown) _rotation_yaw_4)))))))

(fn `UserConstructionScript`)